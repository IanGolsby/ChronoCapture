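; BP_Film is a plane actor that follows the player character at a rotated fixed offset, apparently as a held film for a Chrono Capture feature.
; Each Tick copies the player's location and rotation with the offset applied, then adds a local 90-degree rotation to orient the plane.
; BeginPlay applies the initial capture material, and the Activate Material function swaps it to the ChronoCapture material.
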(event `self.ReceiveTick`
  (params (DeltaSeconds :type "Float (single-precision)"))
  (bind _returnvalue (`GameplayStatics.GetPlayerCharacter` 0))
  (bind _returnvalue_2 (`self.K2_GetActorRotation` _returnvalue))
  (`self.K2_SetActorLocationAndRotation` (+ (`KismetMathLibrary.GreaterGreater_VectorRotator` (150.0 100.0 100.0) _returnvalue_2) (`self.K2_GetActorLocation` _returnvalue)) _returnvalue_2)
  (`self.K2_AddActorLocalRotation` (struct :`Yaw` -90.0)))

(event `self.ReceiveBeginPlay`
  (`PrimitiveComponent.SetMaterial` (`self.Plane`) 0 "/Game/m_ChronoCaptureInitial.m_ChronoCaptureInitial"))

(fn `Activate Material`
  (`PrimitiveComponent.SetMaterial` (`self.Plane`) 0 "/Game/ChronoCapture.ChronoCapture"))

(fn `UserConstructionScript`)
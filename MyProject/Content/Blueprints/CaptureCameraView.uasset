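; CaptureCameraView is a scene capture actor that shadows the player character and takes a snapshot of the view for BP_Film.
; Every tick it moves to a fixed offset far below the player's location and copies the player actor's rotation.
; Its CaptureScene function triggers the SceneCaptureComponent2D, then finds the BP_Film actor by class and calls ActivateMaterial on it.
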(event `self.ReceiveBeginPlay`)

(event `self.ReceiveTick`
  (params (DeltaSeconds :type "Float (single-precision)"))
  (bind _returnvalue (`GameplayStatics.GetPlayerCharacter` 0))
  (`self.K2_SetActorLocationAndRotation` (+ (0.0 0.0 -2600.0) (`self.K2_GetActorLocation` _returnvalue)) (`self.K2_GetActorRotation` _returnvalue))
  (`self.K2_AddActorLocalRotation` (struct)))

(fn `CaptureScene`
  (`SceneCaptureComponent2D.CaptureScene` (`self.SceneCaptureComponent2D`))
  (bind _returnvalue (`GameplayStatics.GetActorOfClass` "/Game/Blueprints/BP_Film.BP_Film_C"))
  (`/Game/Blueprints/BP_Film.Activate Material` _returnvalue))

(fn `UserConstructionScript`)